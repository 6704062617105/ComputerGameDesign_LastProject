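; EnemyCharacter is an enemy with a floating health bar that ragdolls on death.
; Each damage event calls the parent handler, then updates the HealthBar widget cached at BeginPlay with the health percentage.
; At zero health it disables capsule collision, stops movement, hides the bar, launches the physics-simulated mesh with an impulse, and destroys itself after a delay.
; Construction randomizes a dark body color via dynamic material; random run-speed logic is disconnected.
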(event EventBeginPlay
  (bind _ashealth_bar (Utilities|Casting|CastToHealthBar (UserInterface|GetUserWidgetObject (Variables|Default|GetHealthWidget))))
  (Variables|Default|SetHealthBar _ashealth_bar))

(event EventOnReceiveDamage
  (|CallParentFunction)
  (Default|UpdateHealth (Variables|Default|GetHealthBar) (* (/ (Math|Conversions|ToFloat(Integer) (Variables|Default|GetHealth)) (Math|Conversions|ToFloat(Integer) (Variables|Default|GetTotalHealth))) 1e+02))
  (if (<= (Variables|Default|GetHealth) 0)
    (Collision|SetCollisionEnabled (Variables|Default|GetCapsuleComponent) "NoCollision")
    (Components|Movement|StopMovementImmediately (Variables|Character|GetCharacterMovement))
    (Rendering|SetVisibility (Variables|Default|GetHealthWidget) false false)
    (Physics|SetSimulatePhysics (Variables|Character|GetMesh) true)
    (Physics|AddImpulse (Variables|Character|GetMesh) (Math|Conversions|ToVector(Float) (Variables|Default|GetImpulseVelocity)) "None" true)
    (Utilities|FlowControl|Delay 5.0)
    (Actor|DestroyActor)))

(fn ConstructionScript
  (bind _returnvalue (Rendering|Material|CreateDynamicMaterialInstance (Variables|Character|GetMesh) 0 0 "None" :!class /Script/Engine.PrimitiveComponent))
  (bind _output_get (Variables|Default|SetDynamicMaterial _returnvalue))
  (Rendering|Material|SetVectorParameterValue _output_get "BodyColor" (Math|Color|MakeColor (Math|Random|RandomFloatinRange 0.0 0.3) (Math|Random|RandomFloatinRange 0.0 0.3) (Math|Random|RandomFloatinRange 0.0 0.3)) :!class /Script/Engine.MaterialInstanceDynamic))