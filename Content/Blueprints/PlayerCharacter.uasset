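; Player character Blueprint that handles camera-relative movement, look input, and picking up and firing a weapon.
; Overlapping a WeaponPickup spawns a weapon, attaches it to the mesh's GunSocket and sets IsArmed, which gates the Fire input that starts and stops shooting.
; Movement follows the camera's forward and right vectors, while look axes drive controller yaw and pitch.
; An Upgrade event overrides the current weapon's damage with a fixed value.
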(event Custom|Upgrade
  ;[1 1 1] Upgrade Damage
  (bind _output_get (Variables|Default|SetWeapon (Variables|Default|GetWeapon)))
  (Variables|/Game/Blueprints/Weapon.Weapon_C|SetWeaponDamage _output_get 100))

(event Collision|EventActorBeginOverlap
  (params (OtherActor :type Actor%20Object%20Reference))
  (bind _mesh (Variables|Character|GetMesh))
  ;[1 1 1] Spawn Weapon
  (Utilities|Casting|CastToWeaponPickup OtherActor)
  (bind _returnvalue (Game|SpawnActorfromClass "/Game/Blueprints/Weapon.Weapon_C" (Transformation|GetWorldTransform _mesh) "Undefined" 0 0))
  (bind _output_get (Variables|Default|SetWeapon _returnvalue))
  (Transformation|AttachComponentToComponent _output_get _mesh "GunSocket" "SnapToTarget" "SnapToTarget" "SnapToTarget" true)
  (Variables|Default|SetisArmed true))

(event Input|ActionEvents|InputActionFire
  (params (Key :type Key%20Structure :default "None"))
  (bind _weapon (Variables|Default|GetWeapon))
  ;[1 1 1] Fire Weapon
  (:Pressed
    (if (Variables|Default|GetisArmed)
      (Default|FireWeapon _weapon)))
  (:Released
    (if (Variables|Default|GetisArmed)
      (Default|StopFiring _weapon))))

(event Input|AxisEvents|InputAxisMoveUp
  (params (AxisValue :type Float%20%28single-precision%29))
  ;[1 1 1] Movement
  (Pawn|Input|AddMovementInput (Math|Vector|GetForwardVector (Transformation|GetWorldRotation (Variables|Default|GetCamera))) AxisValue false))

(event Input|AxisEvents|InputAxisMoveRight
  (params (AxisValue :type Float%20%28single-precision%29))
  ;[1 1 1] Movement
  (Pawn|Input|AddMovementInput (Math|Vector|GetRightVector (Transformation|GetWorldRotation (Variables|Default|GetCamera))) AxisValue false))

(event Input|AxisEvents|InputAxisLookRight
  (params (AxisValue :type Float%20%28single-precision%29))
  ;[1 1 1] Rotation
  (Pawn|Input|AddControllerYawInput AxisValue))

(event Input|AxisEvents|InputAxisLookUp
  (params (AxisValue :type Float%20%28single-precision%29))
  ;[1 1 1] Rotation
  (Pawn|Input|AddControllerPitchInput AxisValue))

(fn ConstructionScript)