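; A door actor that slides its Door component up when something overlaps it and lowers it again after a short pause.
; On overlap it plays a rifle-shot sound at the actor's location, then chains MoveComponentTo, a delay and a reverse move along relative Z by MoveDistance.
; An IsClosed flag ignores further overlaps until the cycle finishes, with no filter on which actor triggers it.
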(event Collision|EventActorBeginOverlap
  (params (OtherActor :type Actor%20Object%20Reference))
  (bind _door (Variables|Default|GetDoor))
  (bind _door_2 (Variables|Default|GetDoor))
  (bind _relativelocation (Variables|/Script/Engine.SceneComponent|GetRelativeLocation _door))
  (bind _relativelocation_2 (Variables|/Script/Engine.SceneComponent|GetRelativeLocation _door_2))
  (if (Variables|Default|GetIsClosed)
    (Variables|Default|SetIsClosed false)
    (Audio|PlaySoundatLocation "/Game/Assets_External/Audio/AssaultRifle_Shot01_Stereo.AssaultRifle_Shot01_Stereo" (Transformation|GetActorLocation) "0, 0, 0" 1.0 1.0 0.0 0 0 0)
    (Components|MoveComponentTo _door (Math|Vector|MakeVector (.x _relativelocation) (.y _relativelocation) (+ (.z _relativelocation) (Variables|Default|GetMoveDistance))) (Variables|/Script/Engine.SceneComponent|GetRelativeRotation _door) false false 0.2 false)
    (Utilities|FlowControl|Delay 2.0)
    (Components|MoveComponentTo _door_2 (Math|Vector|MakeVector (.x _relativelocation_2) (.y _relativelocation_2) (- (.z _relativelocation_2) (Variables|Default|GetMoveDistance))) (Variables|/Script/Engine.SceneComponent|GetRelativeRotation _door_2) false false 0.2 false)
    (Variables|Default|SetIsClosed true)))

(fn ConstructionScript)