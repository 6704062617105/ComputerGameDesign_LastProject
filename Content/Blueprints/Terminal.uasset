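; Terminal actor that shows a one-time player tip widget when an actor overlaps it while PlayerCanInteract is true.
; The overlap handler creates the PlayerTip widget, adds it to the viewport and removes it after a short delay.
; HasShownTooltip blocks later displays but is set only after that delay, and the overlapping actor's identity is not checked.
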(event EventBeginPlay)

(event Collision|EventActorBeginOverlap
  (params (OtherActor :type Actor%20Object%20Reference))
  (if (and (Variables|Default|GetPlayerCanInteract) (not (Variables|Default|GetHasShownTooltip)))
    (bind _returnvalue (UserInterface|CreateWidget "/Game/UI/PlayerTip.PlayerTip_C"))
    (bind _output_get (Variables|Default|SetPlayerTip _returnvalue))
    (UserInterface|Viewport|AddtoViewport _output_get 0)
    (Utilities|FlowControl|Delay 5.0)
    (Widget|RemovefromParent _output_get)
    (Variables|Default|SetHasShownTooltip true)))

(event EventTick
  (params (DeltaSeconds :type Float%20%28single-precision%29)))

(fn ConstructionScript)