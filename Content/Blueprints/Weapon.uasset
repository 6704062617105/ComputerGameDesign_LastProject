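; Weapon Blueprint for an automatic hitscan gun that damages enemy characters.
; FireWeapon line-traces forward from LaserSpawn, calls ReceiveDamage on an EnemyCharacter hit, spawns enemy or default impact effects, and sets a looping cooldown timer on itself.
; A DoOnce starts the attached muzzle effect and looping fire audio only once per burst.
; StopFiring clears the timer, removes the effect, stops the audio and resets the DoOnce.
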(event Custom|FireWeapon
  (bind _laserspawn (Variables|Default|GetLaserSpawn))
  (bind _laserspawn_2 (Variables|Default|GetLaserSpawn))
  (bind _returnvalue (Transformation|GetWorldLocation _laserspawn))
  ;[1 1 1] Fire Weapon
  (Utilities|FlowControl|Sequence
    (:then_0
      ;[1 1 1] Sound & FX
      (Utilities|FlowControl|DoOnce false ; Play Muzzle FX and Animation Only Once
        (:Completed
          (Utilities|FlowControl|Sequence
            (:then_0
              (bind _returnvalue_2 (Effects|SpawnEmitterAttached "/Game/Assets_External/GunFX/ParticleSystems/Weapons/AssaultRifle/Muzzle/P_AssaultRifle_MF.P_AssaultRifle_MF" _laserspawn_2 "None" (Transformation|GetWorldLocation _laserspawn_2) (Transformation|GetWorldRotation _laserspawn_2) "1.000000,1.000000,1.000000" "KeepWorldPosition" false)))
            (:then_1
              (bind _returnvalue_3 (Audio|SpawnSoundAttached "/Game/Audio/AssaultLoop.AssaultLoop" _laserspawn_2 "None" "0, 0, 0" "0, 0, 0" "KeepRelativeOffset" true 2.0 1.0 0.0 0 0 false))
              (Variables|Default|SetAssaultLoop _returnvalue_3) ; Save as variable so we can destroy later
            )))))
    (:then_1
      ;[1 1 1] Bullets (Raycasting)
      (bind _outhit (Collision|LineTraceByChannel _returnvalue (+ _returnvalue (* (Math|Vector|GetForwardVector (Transformation|GetWorldRotation _laserspawn)) (Math|Conversions|ToVector(Float) (Variables|Default|GetWeaponRange)))) "TraceTypeQuery1" false 0 "ForOneFrame"))
      (bind _output_get (Variables|Default|SetHitActor (.HitActor (Collision|BreakHitResult _outhit))))
      (bind _asenemy_character (Utilities|Casting|CastToEnemyCharacter _output_get)
        (:then
          (Default|ReceiveDamage _asenemy_character (Variables|Default|GetWeaponDamage)) ; Call Receive Damage Function on Enemy
          ;[1 1 1] FX For Bullet Impact
          (Effects|SpawnEmitteratLocation "/Game/FX/EnemyImpact.EnemyImpact" (.ImpactPoint (Collision|BreakHitResult _outhit)) (Math|Conversions|RotationFromXVector (.ImpactNormal (Collision|BreakHitResult _outhit))))
          (Utilities|FlowControl|Delay 0.5))
        (:CastFailed
          (Effects|SpawnEmitteratLocation "/Game/Assets_External/GunFX/ParticleSystems/Weapons/AssaultRifle/Impacts/P_AssaultRifle_IH.P_AssaultRifle_IH" (.ImpactPoint (Collision|BreakHitResult _outhit)) (Math|Conversions|RotationFromXVector (.ImpactNormal (Collision|BreakHitResult _outhit))))
          (Utilities|FlowControl|Delay 0.5)
          (Audio|SpawnSoundatLocation 0 (.ImpactPoint (Collision|BreakHitResult _outhit)) "0, 0, 0" 1.0 1.0 0.0 0 0))))
    (:then_2
      (bind _returnvalue_4 (Utilities|Time|SetTimerbyFunctionName 0 "FireWeapon" (Variables|Default|GetWeaponCooldown) true)) ; Keep calling FireWeapon so Raycasts (bullets) keep firing
    )))

(event Custom|StopFiring
  (bind _laserspawn (Variables|Default|GetLaserSpawn))
  ;[1 1 1] Fire Weapon
  (Utilities|FlowControl|Sequence
    (:then_0
      (Utilities|Time|ClearandInvalidateTimerbyHandle (stale Custom|FireWeapon _returnvalue_4)))
    (:then_1
      ;[1 1 1] Sound & FX
      (Components|DestroyComponent (stale Custom|FireWeapon _returnvalue_2))
      (Audio|Components|Audio|Stop (Variables|Default|GetAssaultLoop)))
    (:then_2
      (Utilities|FlowControl|DoOnce false) ; enters at Reset
    )))

(fn ConstructionScript)