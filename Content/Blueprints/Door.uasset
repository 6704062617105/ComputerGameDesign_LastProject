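; Double sliding door that opens when an actor begins overlapping it and closes again automatically after a short delay.
; An IsClosed flag blocks retriggering while a rifle-shot sound plays and a Sequence slides both panels apart along relative Y by MoveDistance.
; Each branch uses MoveComponentTo, disables collision on the opposite side's components during the wait, then restores it after sliding back.
; Only the left branch resets IsClosed.
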(event Collision|EventActorBeginOverlap
  (params (OtherActor :type Actor%20Object%20Reference))
  (bind _rightdoor (Variables|Default|GetRightDoor))
  (bind _leftdoor (Variables|Default|GetLeftDoor))
  (bind _leftdoor_2 (Variables|Default|GetLeftDoor))
  (bind _rightdoor_2 (Variables|Default|GetRightDoor))
  (bind _relativelocation (Variables|/Script/Engine.SceneComponent|GetRelativeLocation _leftdoor))
  (bind _relativelocation_2 (Variables|/Script/Engine.SceneComponent|GetRelativeLocation _rightdoor))
  (bind _relativelocation_3 (Variables|/Script/Engine.SceneComponent|GetRelativeLocation _rightdoor_2))
  (bind _relativelocation_4 (Variables|/Script/Engine.SceneComponent|GetRelativeLocation _leftdoor_2))
  (if (Variables|Default|GetIsClosed)
    (Variables|Default|SetIsClosed false)
    (Audio|PlaySoundatLocation "/Game/Assets_External/Audio/AssaultRifle_Shot01_Stereo.AssaultRifle_Shot01_Stereo" (Transformation|GetActorLocation) "0, 0, 0" 1.0 1.0 0.0 0 0 0)
    (Utilities|FlowControl|Sequence
      (:then_0
        (Components|MoveComponentTo _rightdoor (Math|Vector|MakeVector (.x _relativelocation_2) (+ (.y _relativelocation_2) (Variables|Default|GetMoveDistance)) (.z _relativelocation_2)) (Variables|/Script/Engine.SceneComponent|GetRelativeRotation _rightdoor) false false 0.2 false)
        (Collision|SetCollisionEnabled (Variables|Default|GetLeftDoor) "NoCollision")
        (Utilities|FlowControl|Delay 2.0)
        (Components|MoveComponentTo _rightdoor_2 (Math|Vector|MakeVector (.x _relativelocation_3) (- (.y _relativelocation_3) (Variables|Default|GetMoveDistance)) (.z _relativelocation_3)) (Variables|/Script/Engine.SceneComponent|GetRelativeRotation _rightdoor_2) false false 0.2 false)
        (Collision|SetCollisionEnabled (Variables|Default|GetLeftDoor) "QueryAndPhysics"))
      (:then_1
        (Components|MoveComponentTo _leftdoor (Math|Vector|MakeVector (.x _relativelocation) (- (.y _relativelocation) (Variables|Default|GetMoveDistance)) (.z _relativelocation)) (Variables|/Script/Engine.SceneComponent|GetRelativeRotation _leftdoor) false false 0.2 false)
        (Collision|SetCollisionEnabled (Variables|Default|GetRightDoor1) "NoCollision")
        (Utilities|FlowControl|Delay 2.0)
        (Components|MoveComponentTo _leftdoor_2 (Math|Vector|MakeVector (.x _relativelocation_4) (+ (.y _relativelocation_4) (Variables|Default|GetMoveDistance)) (.z _relativelocation_4)) (Variables|/Script/Engine.SceneComponent|GetRelativeRotation _leftdoor_2) false false 0.2 false)
        (Variables|Default|SetIsClosed true)
        (Collision|SetCollisionEnabled (Variables|Default|GetRightDoor1) "QueryAndPhysics")))))

(event EventTick
  (params (DeltaSeconds :type Float%20%28single-precision%29)))

(fn ConstructionScript)